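; Multiplayer game mode that registers joining players and respawns them in vehicles at numbered spawn points.
; On authority, PostLogin collects PlayerStarts tagged mp_spawn, sets each GS_PS player number from the PlayerArray length for consistent scoreboard order, then calls ClientPostLogin on PC_MP.
; RespawnPlayerEvent destroys an existing pawn, spawns Vehicle_001_Blueprint at the spawn indexed by player number, and possesses it after a brief delay.
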(event `RespawnPlayerEvent`
  (params (playController :type "PlayerController Object Reference"))
  (bind _returnvalue (`Controller.K2_GetPawn` playController))
  ;[1 1 1] Spawns players at spawns based on player number
  (`/Engine/EditorBlueprintResources/StandardMacros.IsValid` _returnvalue
    (:`Is Valid`
      (`self.K2_DestroyActor` _returnvalue)
      (bind _asgs_ps (cast `/Game/Multiplayer/Blueprints/GS_PS` (`Controller.PlayerState` playController)))
      (bind _returnvalue_2 (`|SpawnActorFromClass` "/Game/Vehicle/Blueprint/Vehicle_001_Blueprint.Vehicle_001_Blueprint_C" (`self.GetTransform` (`KismetArrayLibrary.Array_Get` (`self.mp_spawn`) (`/Game/Multiplayer/Blueprints/GS_PS.playerNumber` _asgs_ps))) "AdjustIfPossibleButAlwaysSpawn" "OverrideRootScale"))
      (`KismetSystemLibrary.Delay` 0.01)
      (`Controller.Possess` playController _returnvalue_2))))

(event `self.ReceiveBeginPlay`)

(event `self.ReceiveTick`
  (params (DeltaSeconds :type "Float (single-precision)")))

(event `self.K2_PostLogin`
  (params (NewPlayer :type "PlayerController Object Reference"))
  ;[1 1 1] post login
  (`/Engine/EditorBlueprintResources/ActorMacros.Switch Has Authority`
    (:`Authority`
      (bind _outactors (`GameplayStatics.GetAllActorsOfClass` "/Script/Engine.PlayerStart"))
      (for _array_element _outactors
        (if (== (`PlayerStart.PlayerStartTag` _array_element) "mp_spawn")
          (`KismetArrayLibrary.Array_AddUnique` (`self.mp_spawn`) _array_element)))
      (bind _asgs_ps (cast `/Game/Multiplayer/Blueprints/GS_PS` (`Controller.PlayerState` NewPlayer)))
      ;;[1 1 1] Verifies the scoreboard will be same order for all players
      (set `/Game/Multiplayer/Blueprints/GS_PS.playerNumber` (`KismetArrayLibrary.Array_Length` (`GameState.PlayerArray` (`GameplayStatics.GetGameState`))) _asgs_ps)
      (bind _aspc_mp (cast `/Game/Multiplayer/Blueprints/PC_MP` NewPlayer))
      (`/Game/Multiplayer/Blueprints/PC_MP.ClientPostLogin` _aspc_mp))))

(fn `UserConstructionScript`)