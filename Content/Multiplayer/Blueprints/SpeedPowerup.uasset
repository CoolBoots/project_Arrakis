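; SpeedPowerup is a pickup that temporarily boosts the movement speed of the SPP_Character that overlaps it.
; On overlap it destroys its collision and sphere components, then casts the other actor, so any overlapping actor consumes it.
; For a character it multiplies MoveSpeed by SpeedMultiple, restores the saved value after a fixed five-second delay and destroys itself.
; The graph contains no authority check and prints on-screen debug messages.
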(event `self.ReceiveBeginPlay`)

(event `self.ReceiveActorBeginOverlap`
  (params (OtherActor :type "Actor Object Reference"))
  (`ActorComponent.K2_DestroyComponent` (`self.SphereCollision`))
  (`ActorComponent.K2_DestroyComponent` (`self.Sphere`))
  (`KismetSystemLibrary.PrintString` "SPEED")
  (bind _asspp_character (cast `/Game/Multiplayer/Blueprints/SPP_Character` OtherActor))
  (bind _output_get (set `self.OriginalSpeed` (`/Game/Multiplayer/Blueprints/SPP_Character.MoveSpeed` _asspp_character)))
  (bind _output_get_2 (set `/Game/Multiplayer/Blueprints/SPP_Character.MoveSpeed` (* (stale _output_get_2) (`self.SpeedMultiple`)) _asspp_character))
  (`KismetSystemLibrary.Delay` 5.0)
  (set `/Game/Multiplayer/Blueprints/SPP_Character.MoveSpeed` _output_get _asspp_character)
  (`KismetSystemLibrary.PrintString` "Speed off")
  (`self.K2_DestroyActor`))

(event `self.ReceiveActorBeginOverlap`
  (params (OtherActor :type "Actor Object Reference")))

(event `self.ReceiveTick`
  (params (DeltaSeconds :type "Float (single-precision)")))

(fn `UserConstructionScript`)