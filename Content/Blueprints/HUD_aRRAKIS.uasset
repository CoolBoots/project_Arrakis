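; HUD Blueprint that draws a yellow timer and speed readout at fixed screen coordinates.
; Time is a counter that Tick increments through a one-second Delay, so it counts roughly in seconds.
; Speed is the player pawn's displacement since the previous DrawHUD call minus a small constant, so it is per frame rather than per second.
; BeginPlay seeds the stored position, which DrawHUD refreshes after each draw.
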(event `self.ReceiveDrawHUD`
  (params (SizeX :type Integer) (SizeY :type Integer))
  (bind _returnvalue (`self.K2_GetActorLocation` (`GameplayStatics.GetPlayerPawn` 0)))
  ;[1 1 1] Timer
  (`self.DrawText` (`KismetStringLibrary.Conv_IntToString` (`self.timeCounter`)) (struct :`R` 1.0 :`G` 0.789766 :`A` 1.0) 1160.0 40.0 "/Engine/EngineFonts/RobotoDistanceField.RobotoDistanceField")
  (`self.DrawText` "Time :" (struct :`R` 1.0 :`G` 0.789766 :`A` 1.0) 1050.0 40.0 "/Engine/EngineFonts/RobotoDistanceField.RobotoDistanceField")
  ;[1 1 1] Speedometer
  (`self.DrawText` (`KismetStringLibrary.Conv_DoubleToString` (- (`KismetMathLibrary.VSize` (- _returnvalue (`self.positionOld`))) 0.035)) (struct :`R` 1.0 :`G` 0.789766 :`A` 1.0) 1160.0 70.0 "/Engine/EngineFonts/RobotoDistanceField.RobotoDistanceField")
  (`self.DrawText` "Speed :" (struct :`R` 1.0 :`G` 0.789766 :`A` 1.0) 1050.0 70.0 "/Engine/EngineFonts/RobotoDistanceField.RobotoDistanceField")
  (set `self.positionOld` _returnvalue))

(event `self.ReceiveTick`
  (params (DeltaSeconds :type "Float (single-precision)"))
  ;[1 1 1] Timer
  (`KismetSystemLibrary.Delay` 1.0)
  (set `self.timeCounter` (+ (`self.timeCounter`) 1)))

(event `self.ReceiveBeginPlay`)

(event `self.ReceiveBeginPlay`
  ;[1 1 1] Speedometer
  ;;[1 1 1] Set original position
  (set `self.positionOld` (`self.K2_GetActorLocation` (`GameplayStatics.GetPlayerPawn` 0))))

(event `self.ReceiveActorBeginOverlap`
  (params (OtherActor :type "Actor Object Reference")))

(event `self.ReceiveTick`
  (params (DeltaSeconds :type "Float (single-precision)")))

(fn `UserConstructionScript`)