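; Drivable vehicle pawn with swappable parts, a placeholder boost and preset camera views.
; Input axes and handbrake drive VehicleMovement; boost multiplies physics velocity and decrements BoostAmount without checking it.
; Randomize replaces spawned parts with classes picked from random level actors, attaching hubcaps and wheels to bone sockets (first two Y-mirrored) and single parts to the player pawn's root.
; Number keys snap the camera to chase, rear-view or cinematic marker transforms.
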(event `InputAxis|Foreward`
  (params (AxisValue :type "Float (single-precision)"))
  ;[1 1 1] Input
  (`WheeledVehicleMovementComponent.SetThrottleInput` (`self.VehicleMovement`) AxisValue))

(event `Key|One`
  (params (Key :type "Key Structure" :default "AnyKey"))
  (bind _cam_chase_cam (`self.CAM_Chase Cam`))
  ;[0.2728 0.291 1] Camera Behaviour
  ;;[1 1 1] Chase Cam - Default camera
  (:`Pressed`
    (`SceneComponent.K2_SetRelativeLocation` (`self.Camera`) (`SceneComponent.RelativeLocation` _cam_chase_cam) false false)
    (`SceneComponent.K2_SetRelativeRotation` (`self.Camera`) (`SceneComponent.RelativeRotation` _cam_chase_cam) false false)))

(event `InputAxis|Left_Right`
  (params (AxisValue :type "Float (single-precision)"))
  ;[1 1 1] Input
  (`WheeledVehicleMovementComponent.SetSteeringInput` (`self.VehicleMovement`) AxisValue))

(event `InputAction|Handbrake`
  (params (Key :type "Key Structure" :default "AnyKey"))
  (bind _vehiclemovement (`self.VehicleMovement`))
  ;[1 1 1] Input
  (:`Pressed`
    (`WheeledVehicleMovementComponent.SetHandbrakeInput` _vehiclemovement true))
  (:`Released`
    (`WheeledVehicleMovementComponent.SetHandbrakeInput` _vehiclemovement false)))

(event `Key|Two`
  (params (Key :type "Key Structure" :default "AnyKey"))
  (bind _cam_rear_view (`self.CAM_Rear View`))
  ;[0.2728 0.291 1] Camera Behaviour
  ;;[1 1 1] Rear-View Mirror Cam - Default look behind camera
  (:`Pressed`
    (`SceneComponent.K2_SetRelativeLocation` (`self.Camera`) (`SceneComponent.RelativeLocation` _cam_rear_view) false false)
    (`SceneComponent.K2_SetRelativeRotation` (`self.Camera`) (`SceneComponent.RelativeRotation` _cam_rear_view) false false)))

(event `InputAction|Boost`
  (params (Key :type "Key Structure" :default "AnyKey"))
  (bind _updatedprimitive (`MovementComponent.UpdatedPrimitive` (`self.VehicleMovement`)))
  ;[1 1 1] Boost: Placeholder. Very Hacky.
  (:`Pressed`
    (bind _returnvalue (`PrimitiveComponent.GetPhysicsLinearVelocity` _updatedprimitive "None"))
    (`PrimitiveComponent.SetPhysicsLinearVelocity` _updatedprimitive (* _returnvalue 1.4) false "None")
    (set `self.boostAmount` (- (`self.boostAmount`) 1))))

(event `InputAction|Randomize`
  (params (Key :type "Key Structure" :default "AnyKey"))
  (bind _arrayactor_selectedvehiclecomponents (`self.arrayActor_SelectedVehicleComponents`))
  ;[1 1 1] Randomisation For Wheel, Hubcaps,Engine and Chassis.
  (:`Pressed`
    (`self.K2_DestroyActor` _arrayactor_selectedvehiclecomponents)
    (`KismetArrayLibrary.Array_Clear` _arrayactor_selectedvehiclecomponents)
    (for (_array_element _array_index) (`self.arrayClass_VehicleComponents_MULTI`)
      (bind _outactors (`GameplayStatics.GetAllActorsOfClass` _array_element))
      (`|MultiGate` false false _array_index :!label _label
        (:`Out 0`
          (set `self.arrayString_BoneNames` (`self.arrayString_HubcapBoneNames`)))
        (:`Out 1`
          (set `self.arrayString_BoneNames` (`self.arrayString_WheelBoneNames`))))
      (bind _output_get (set `self.varibleActor_CurrentVehicleComponent` (`KismetArrayLibrary.Array_Get` _outactors (`KismetMathLibrary.RandomIntegerInRange` 0 (`KismetArrayLibrary.Array_LastIndex` _outactors)))))
      (for (_array_element_2 _array_index_2) (`self.arrayString_BoneNames`)
        (`/Engine/EditorBlueprintResources/StandardMacros.CompareInt` _array_index_2 2
          (:`>`
            _)
          (:`==`
            _)
          (:`<`
            (bind _returnvalue (`GameplayStatics.GetObjectClass` _output_get))
            (bind _returnvalue_2 (`|SpawnActorFromClass` _returnvalue (`KismetMathLibrary.MakeTransform` (0.0 0.0 0.0) (struct) (1.0 -1.0 1.0)) "AlwaysSpawn" "OverrideRootScale"))
            (`KismetArrayLibrary.Array_Add` (`self.arrayActor_SelectedVehicleComponents`) _returnvalue_2)
            (`self.K2_AttachRootComponentToActor` _returnvalue_2 (`GameplayStatics.GetPlayerPawn` 0) (`KismetStringLibrary.Conv_StringToName` _array_element_2) "SnapToTarget" true)
            (goto _label :!via `Reset`)))
        (bind _returnvalue_3 (`|SpawnActorFromClass` _returnvalue (`KismetMathLibrary.MakeTransform` (0.0 0.0 0.0) (struct) (1.0 1.0 1.0)) "AlwaysSpawn" "OverrideRootScale"))
        (`KismetArrayLibrary.Array_Add` (`self.arrayActor_SelectedVehicleComponents`) _returnvalue_3)
        (`self.K2_AttachRootComponentToActor` _returnvalue_3 (`GameplayStatics.GetPlayerPawn` 0) (`KismetStringLibrary.Conv_StringToName` _array_element_2) "SnapToTarget" true)))
    (for _array_element_3 (`self.arrayClass_VehicleComponents_SINGLE`)
      (bind _outactors_2 (`GameplayStatics.GetAllActorsOfClass` _array_element_3))
      (bind _output_get_2 (set `self.varibleActor_CurrentVehicleComponent` (`KismetArrayLibrary.Array_Get` _outactors_2 (`KismetMathLibrary.RandomIntegerInRange` 0 (`KismetArrayLibrary.Array_LastIndex` _outactors_2)))))
      (bind _returnvalue_4 (`|SpawnActorFromClass` (`GameplayStatics.GetObjectClass` _output_get_2) (`KismetMathLibrary.MakeTransform` (0.0 0.0 0.0) (struct) (1.0 1.0 1.0)) "AlwaysSpawn" "OverrideRootScale"))
      (`KismetArrayLibrary.Array_Add` (`self.arrayActor_SelectedVehicleComponents`) _returnvalue_4)
      (`self.K2_AttachRootComponentToActor` _returnvalue_4 (`GameplayStatics.GetPlayerPawn` 0) "None" "SnapToTarget" true))))

(event `Key|Three`
  (params (Key :type "Key Structure" :default "AnyKey"))
  (bind _cam_cinematic_wheel (`self.CAM_Cinematic Wheel`))
  ;[0.2728 0.291 1] Camera Behaviour
  ;;[1 1 1] Wheel cam - Cinematic camera
  (:`Pressed`
    (`SceneComponent.K2_SetRelativeLocation` (`self.Camera`) (`SceneComponent.RelativeLocation` _cam_cinematic_wheel) false false)
    (`SceneComponent.K2_SetRelativeRotation` (`self.Camera`) (`SceneComponent.RelativeRotation` _cam_cinematic_wheel) false false)))

(event `Key|Four`
  (params (Key :type "Key Structure" :default "AnyKey"))
  (bind _cam_cinematic_rear_view (`self.CAM_Cinematic Rear View`))
  ;[0.2728 0.291 1] Camera Behaviour
  ;;[1 1 1] Rear-Facing Front cam - Cinematic camera
  (:`Pressed`
    (`SceneComponent.K2_SetRelativeLocation` (`self.Camera`) (`SceneComponent.RelativeLocation` _cam_cinematic_rear_view) false false)
    (`SceneComponent.K2_SetRelativeRotation` (`self.Camera`) (`SceneComponent.RelativeRotation` _cam_cinematic_rear_view) false false)))

(fn `OnRep_varibleActor_CurrentVehicleComponent`)

(fn `Spawn Part`)

(fn `UserConstructionScript`)